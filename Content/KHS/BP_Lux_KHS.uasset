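; Player character Lux with MOBA-style controls: cursor-driven movement, basic attack, Q/W/E/R skills and mouse-wheel camera zoom.
; Holding right mouse opens a Tick gate that turns toward the cursor, then moves to the point or clicked pawn, attacking instead if any enemy overlaps AttackRange.
; Attacks and skills spawn actors at AttackDir, with W also attaching a barrier; IsAttacking blocks other actions until the montage delay ends.
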(event OnComponentBeginOverlap(AttackRange)
  (params (OverlappedComponent :type Primitive%20Component%20Object%20Reference) (OtherActor :type Actor%20Object%20Reference) (OtherComp :type Primitive%20Component%20Object%20Reference) (OtherBodyIndex :type Integer) (bFromSweep :type Boolean) (SweepResult :type Hit%20Result%20Structure%20%28by%20ref%29))
  ;[1 1 1] 우클릭으로 이동 & 평타(사거리 550)
  (Utilities|Casting|CastToBP_Enemy OtherActor)
  (Variables|Default|SetEnemy%20In%20Attack%20Range true))

(event OnComponentEndOverlap(AttackRange)
  (params (OverlappedComponent :type Primitive%20Component%20Object%20Reference) (OtherActor :type Actor%20Object%20Reference) (OtherComp :type Primitive%20Component%20Object%20Reference) (OtherBodyIndex :type Integer))
  ;[1 1 1] 우클릭으로 이동 & 평타(사거리 550)
  (Utilities|Casting|CastToBP_Enemy OtherActor)
  (Variables|Default|SetEnemy%20In%20Attack%20Range false))

(event Custom|Attack
  ;[1 1 1] 우클릭으로 이동 & 평타(사거리 550)
  (if (not (Variables|Default|GetIs%20Attacking?))
    (Variables|Default|SetIs%20Attacking? true)
    (Components|Movement|StopMovementImmediately (Variables|Character|GetCharacterMovement))
    (bind _returnvalue (Game|SpawnActorfromClass "/Game/JSH/Blueprints/SKILL/BP_QQQ.BP_QQQ_C" (Transformation|GetWorldTransform (Variables|Default|GetAttack%20Dir)) "Undefined" "MultiplyWithRoot" 0 0))
    (Variables|/Game/JSH/Blueprints/SKILL/BP_QQQ.BP_QQQ_C|SetAttackOwner _returnvalue self)
    (bind _returnvalue_2 (Animation|PlayAnimMontage 0 1.0 ""))
    (Utilities|FlowControl|Delay _returnvalue_2)
    (Variables|Default|SetIs%20Attacking? false)))

(event EventTick
  (params (DeltaSeconds :type Float%20%28single-precision%29))
  ;[1 1 1] 우클릭으로 이동 & 평타(사거리 550)
  (Utilities|FlowControl|Gate true
    (:Exit
      (if (not (Variables|Default|GetIs%20Attacking?))
        (CallFunction|TurnAttackDir)
        (bind _clicked_actor (CallFunction|GetClickedActor))
        (Utilities|IsValid _clicked_actor
          (:Is%20Valid
            (if (Variables|Default|GetEnemy%20In%20Attack%20Range)
              (CallFunction|Attack)
              (else
                (CallFunction|MovetoActor _clicked_actor))))
          (:Is%20Not%20Valid
            (CallFunction|MovetoClickedPoint)))))))

(event EventBeginPlay
  ;[1 1 1] 마우스 커서 보이기
  (Variables|/Script/Engine.PlayerController|SetbShowMouseCursor (Game|GetPlayerController 0) true))

(event Input|MouseEvents|MouseWheelAxis
  (params (AxisValue :type Float%20%28single-precision%29))
  ;[1 1 1] 마우스 휠로 Zoom in/Out
  (Variables|/Script/Engine.SpringArmComponent|SetTargetArmLength (Variables|Default|GetSpringArm) (Math|Float|Clamp(Float) (+ (* AxisValue -2e+01) (Variables|/Script/Engine.SpringArmComponent|GetTargetArmLength (Variables|Default|GetSpringArm))) 5e+01 1e+03)))

(event Input|MouseEvents|RightMouseButton
  (params (Key :type Key%20Structure :default "None"))
  ;[1 1 1] 우클릭으로 이동 & 평타(사거리 550)
  (:Pressed
    (Utilities|FlowControl|Gate true) ; enters at Open
  )
  (:Released
    (Utilities|FlowControl|Gate true) ; enters at Close
  ))

(event Input|KeyboardEvents|Q
  (params (Key :type Key%20Structure :default "None"))
  ;[1 1 1] 스킬 Q
  (:Pressed
    (if (not (Variables|Default|GetIs%20Attacking?))
      (Variables|Default|SetIs%20Attacking? true)
      (Components|Movement|StopMovementImmediately (Variables|Character|GetCharacterMovement))
      (CallFunction|TurnAttackDir)
      (Game|SpawnActorfromClass "/Game/JSH/Blueprints/SKILL/BP_QQQ.BP_QQQ_C" (Transformation|GetWorldTransform (Variables|Default|GetAttack%20Dir)) "AlwaysSpawn" "MultiplyWithRoot" 0 0)
      (bind _returnvalue (Animation|PlayAnimMontage 0 1.0 "None"))
      (Utilities|FlowControl|Delay _returnvalue)
      (Variables|Default|SetIs%20Attacking? false))))

(event Input|KeyboardEvents|R
  (params (Key :type Key%20Structure :default "None"))
  ;[1 1 1] 스킬 R
  (:Pressed
    (if (not (Variables|Default|GetIs%20Attacking?))
      (Variables|Default|SetIs%20Attacking? true)
      (Components|Movement|StopMovementImmediately (Variables|Character|GetCharacterMovement))
      (CallFunction|TurnAttackDir)
      (Game|SpawnActorfromClass "/Game/JSH/Blueprints/SKILL/BP_RRR.BP_RRR_C" (Transformation|GetWorldTransform (Variables|Default|GetAttack%20Dir)) "AlwaysSpawn" "MultiplyWithRoot" 0 0)
      (bind _returnvalue (Animation|PlayAnimMontage 0 1.0 "None"))
      (Utilities|FlowControl|Delay _returnvalue)
      (Variables|Default|SetIs%20Attacking? false))))

(event Input|KeyboardEvents|W
  (params (Key :type Key%20Structure :default "None"))
  ;[1 1 1] 스킬 W
  (:Pressed
    (if (not (Variables|Default|GetIs%20Attacking?))
      (Variables|Default|SetIs%20Attacking? true)
      (Components|Movement|StopMovementImmediately (Variables|Character|GetCharacterMovement))
      (CallFunction|TurnAttackDir)
      (bind _returnvalue (Game|SpawnActorfromClass "/Game/JSH/Blueprints/SKILL/BP_Barrier.BP_Barrier_C" (Math|Transform|MakeTransform (Transformation|GetActorLocation) "0, 0, 0" "1.000000,1.000000,1.000000") "AlwaysSpawn" "MultiplyWithRoot" 0 0))
      (Transformation|AttachActorToActor _returnvalue self "None" "SnapToTarget" "SnapToTarget" "KeepWorld" true)
      (Game|SpawnActorfromClass "/Game/JSH/Blueprints/SKILL/BP_WWW.BP_WWW_C" (Transformation|GetWorldTransform (Variables|Default|GetAttack%20Dir)) "AlwaysSpawn" "MultiplyWithRoot" 0 0)
      (bind _returnvalue_2 (Animation|PlayAnimMontage 0 1.0 "None"))
      (Utilities|FlowControl|Delay _returnvalue_2)
      (Variables|Default|SetIs%20Attacking? false))))

(event Input|KeyboardEvents|E
  (params (Key :type Key%20Structure :default "None"))
  ;[1 1 1] 스킬 E
  (:Pressed
    (if (not (Variables|Default|GetIs%20Attacking?))
      (Variables|Default|SetIs%20Attacking? true)
      (Components|Movement|StopMovementImmediately (Variables|Character|GetCharacterMovement))
      (CallFunction|TurnAttackDir)
      (Game|SpawnActorfromClass "/Game/JSH/Blueprints/SKILL/BP_E.BP_E_C" (Transformation|GetWorldTransform (Variables|Default|GetAttack%20Dir)) "AlwaysSpawn" "MultiplyWithRoot" 0 0)
      (bind _returnvalue (Animation|PlayAnimMontage 0 1.0 "None"))
      (Utilities|FlowControl|Delay _returnvalue)
      (Variables|Default|SetIs%20Attacking? false))))

(fn ConstructionScript)

(fn GetClickedActor
  (return (.hitactor (.HitResult (Class|PlayerController|GetHitResultUnderCursorforObjects (Game|GetPlayerController 0) (Utilities|Array|MakeArray "ObjectTypeQuery3") true)))))

(fn MovetoActor
  (params (Move%20to%20Actor :type Actor%20Object%20Reference))
  (AI|Navigation|SimpleMovetoActor (Game|GetPlayerController 0) Move%20to%20Actor))

(fn GetDestinationtoMove
  (return (.location (.HitResult (Game|Player|GetHitResultUnderCursorbyChannel (Game|GetPlayerController 0) "TraceTypeQuery1" true)))))

(fn MovetoClickedPoint
  (bind _charactermovement (Variables|Character|GetCharacterMovement))
  (bind _destination (CallFunction|GetDestinationtoMove))
  (Variables|Default|SetMove%20Destination _destination)
  (if (> (Math|Vector|VectorLength (- (Variables|Default|GetMove%20Destination) (Transformation|GetActorLocation))) 1.5e+02)
    (Variables|/Script/Engine.CharacterMovementComponent|SetMaxWalkSpeed _charactermovement 6e+02)
    (else
      (Variables|/Script/Engine.CharacterMovementComponent|SetMaxWalkSpeed _charactermovement 1.5e+02)))
  (AI|Navigation|SimpleMovetoLocation (Game|GetPlayerController 0) (Variables|Default|GetMove%20Destination)))

(fn TurnAttackDir
  (bind _returnvalue (Transformation|GetActorRotation))
  (Transformation|SetActorRotation (Math|Rotator|MakeRotator (.roll _returnvalue) (.pitch _returnvalue) (.yaw (Math|Rotator|FindLookatRotation (+ "" "") (- (.ImpactPoint (Collision|BreakHitResult (.HitResult (Game|Player|GetHitResultUnderCursorbyChannel (Game|GetPlayerController 0) "TraceTypeQuery1" true)))) (Transformation|GetActorLocation)))))))