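; BP_DummyGaren is a test champion with League-style click controls, a visible cursor and mouse-wheel spring-arm zoom.
; Holding right mouse opens a Tick gate to attack or move, but its targeting and movement functions are empty stubs.
; AttackRange overlaps with BP_Enemy set the range flag and trigger Attack, which stops movement and spawns BP_BasicAttack behind an IsAttacking lock.
; Q spawns BP_Q under the cursor; W, E and R only play montages.
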(event OnComponentBeginOverlap(AttackRange)
  (params (OverlappedComponent :type Primitive%20Component%20Object%20Reference) (OtherActor :type Actor%20Object%20Reference) (OtherComp :type Primitive%20Component%20Object%20Reference) (OtherBodyIndex :type Integer) (bFromSweep :type Boolean) (SweepResult :type Hit%20Result%20Structure%20%28by%20ref%29))
  ;[1 1 1] 우클릭으로 이동 & 평타(사거리 550)
  (Utilities|Casting|CastToBP_Enemy OtherActor)
  (Variables|Default|SetEnemyinAttackRange true)
  (CallFunction|Attack))

(event OnComponentEndOverlap(AttackRange)
  (params (OverlappedComponent :type Primitive%20Component%20Object%20Reference) (OtherActor :type Actor%20Object%20Reference) (OtherComp :type Primitive%20Component%20Object%20Reference) (OtherBodyIndex :type Integer))
  ;[1 1 1] 우클릭으로 이동 & 평타(사거리 550)
  (Utilities|Casting|CastToBP_Enemy OtherActor)
  (Variables|Default|SetEnemyinAttackRange false))

(event Custom|Attack
  ;[1 1 1] 우클릭으로 이동 & 평타(사거리 550)
  (if (not (Variables|Default|GetIsAttacking?))
    (Variables|Default|SetIsAttacking? true)
    (Components|Movement|StopMovementImmediately (Variables|Character|GetCharacterMovement))
    (Game|SpawnActorfromClass "/Game/JSH/Blueprints/BP_BasicAttack.BP_BasicAttack_C" (Transformation|GetWorldTransform (Variables|Default|GetAttackDir)) "AlwaysSpawn" "MultiplyWithRoot" 0 0)
    (bind _returnvalue (Animation|PlayAnimMontage 0 1.0 ""))
    (Utilities|FlowControl|Delay _returnvalue)
    (Variables|Default|SetIsAttacking? false)))

(event EventTick
  (params (DeltaSeconds :type Float%20%28single-precision%29))
  ;[1 1 1] 우클릭으로 이동 & 평타(사거리 550)
  (Utilities|FlowControl|Gate true
    (:Exit
      (bind _clicked_actor (CallFunction|GetClickedActor))
      (Utilities|IsValid _clicked_actor
        (:Is%20Valid
          (if (Variables|Default|GetEnemyinAttackRange)
            (CallFunction|Attack)
            (else
              (CallFunction|MovetoActor _clicked_actor))))
        (:Is%20Not%20Valid
          (CallFunction|MovetoClickedPoint))))))

(event Collision|EventActorBeginOverlap
  (params (OtherActor :type Actor%20Object%20Reference))
  ;[1 1 1] QWER 스킬 애니메이션
)

(event EventBeginPlay
  ;[1 1 1] 마우스 커서 보이기
  (Variables|/Script/Engine.PlayerController|SetbShowMouseCursor (Game|GetPlayerController 0) true))

(event Input|MouseEvents|MouseWheelAxis
  (params (AxisValue :type Float%20%28single-precision%29))
  ;[1 1 1] 마우스 휠로 Zoom in/Out
  (Variables|/Script/Engine.SpringArmComponent|SetTargetArmLength (Variables|Default|GetSpringArm) (Math|Float|Clamp(Float) (+ (* AxisValue -2e+01) (Variables|/Script/Engine.SpringArmComponent|GetTargetArmLength (Variables|Default|GetSpringArm))) 5e+01 1e+03)))

(event Input|KeyboardEvents|Q
  (params (Key :type Key%20Structure :default "None"))
  (:Pressed
    (Game|SpawnActorfromClass "/Game/JSH/Blueprints/BP_Q.BP_Q_C" (Math|Transform|MakeTransform (.Location (Collision|BreakHitResult (.HitResult (Game|Player|GetHitResultUnderCursorbyChannel (Game|GetPlayerController 0) "TraceTypeQuery1" true)))) (Transformation|GetWorldRotation (Variables|Default|GetAttackRange))) "AlwaysSpawn" "MultiplyWithRoot" 0 0)
    (Animation|Montage|PlayMontage (Variables|Character|GetMesh) 0
      (:then
        (Utilities|FlowControl|Delay 0.2)
        (Variables|Default|SetIsAttacking? false)))))

(event Input|MouseEvents|RightMouseButton
  (params (Key :type Key%20Structure :default "None"))
  ;[1 1 1] 우클릭으로 이동 & 평타(사거리 550)
  (:Pressed
    (Utilities|FlowControl|Gate true) ; enters at Open
  )
  (:Released
    (Utilities|FlowControl|Gate true) ; enters at Close
  ))

(event Input|KeyboardEvents|W
  (params (Key :type Key%20Structure :default "None"))
  ;[1 1 1] QWER 스킬 애니메이션
  (:Pressed
    (Animation|Montage|PlayMontage (Variables|Character|GetMesh) 0)))

(event Input|KeyboardEvents|E
  (params (Key :type Key%20Structure :default "None"))
  ;[1 1 1] QWER 스킬 애니메이션
  (:Pressed
    (Animation|Montage|PlayMontage (Variables|Character|GetMesh) 0)))

(event Input|KeyboardEvents|R
  (params (Key :type Key%20Structure :default "None"))
  ;[1 1 1] QWER 스킬 애니메이션
  (:Pressed
    (Animation|Montage|PlayMontage (Variables|Character|GetMesh) 0)))

(fn ConstructionScript)

(fn GetClickedActor
  (return 0))

(fn MovetoActor
  (params (Move%20to%20Actor :type Actor%20Object%20Reference)))

(fn MovetoClickedPoint)