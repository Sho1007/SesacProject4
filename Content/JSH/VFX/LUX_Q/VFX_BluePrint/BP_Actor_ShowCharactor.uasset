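; Actor that plays a character reveal effect, pairing a Niagara system with a rising Cube.
; On BeginPlay or a J press, it repositions the Cube, replaces any existing Niagara system with one spawned near ground height, and enables movement for a few seconds.
; While enabled, Tick raises the Cube at constant speed, forcing its world X and Y to zero.
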(event EventBeginPlay
  (bind _self self)
  (bind _self_2 self)
  (bind _returnvalue (Transformation|GetActorLocation _self))
  (bind _returnvalue_2 (Transformation|GetActorLocation _self_2))
  (bind (_x _y) (Math|Vector|BreakVector _returnvalue))
  (bind (_x_2 _y_2) (Math|Vector|BreakVector _returnvalue_2))
  (Input|EnableInput self (Game|GetPlayerController 0))
  (Variables|Default|SetstartMove false)
  ;[1 1 1] Add new Niagara system
  (Transformation|SetRelativeLocation (Variables|Default|GetCube) (Math|Vector|MakeVector _x_2 _y_2 0.0) false false)
  (Utilities|IsValid (Variables|Default|GetngSystemObj)
    (:Is%20Valid
      (Components|DestroyComponent (Variables|Default|GetngSystemObj)))
    (:Is%20Not%20Valid
      _))
  (bind _returnvalue_3 (Niagara|SpawnSystematLocation 0 (Math|Vector|MakeVector _x _y 0.1)))
  (Variables|Default|SetngSystemObj _returnvalue_3)
  (Variables|Default|SetstartMove true)
  (Utilities|FlowControl|Delay 6.0)
  (Variables|Default|SetstartMove false))

(event Collision|EventActorBeginOverlap
  (params (OtherActor :type Actor%20Object%20Reference)))

(event EventTick
  (params (DeltaSeconds :type Float%20%28single-precision%29))
  (bind _cube (Variables|Default|GetCube))
  ;[1 1 1] Move Cube up to show charactor
  (if (Variables|Default|GetstartMove)
    (Transformation|SetWorldLocation _cube (Math|Vector|MakeVector 0.0 0.0 (+ (.Z (Math|Vector|BreakVector (Transformation|GetWorldLocation _cube))) (* DeltaSeconds 65.0))) false false)))

(event Input|KeyboardEvents|J
  (params (Key :type Key%20Structure))
  (bind _self self)
  (bind _self_2 self)
  (bind _returnvalue (Transformation|GetActorLocation _self))
  (bind _returnvalue_2 (Transformation|GetActorLocation _self_2))
  (bind (_x _y) (Math|Vector|BreakVector _returnvalue))
  (bind (_x_2 _y_2) (Math|Vector|BreakVector _returnvalue_2))
  ;[1 1 1] push key J
  (:Pressed
    ;[1 1 1] Add new Niagara system
    (Transformation|SetRelativeLocation (Variables|Default|GetCube) (Math|Vector|MakeVector _x_2 _y_2 0.0) false false)
    (Utilities|IsValid (Variables|Default|GetngSystemObj)
      (:Is%20Valid
        (Components|DestroyComponent (Variables|Default|GetngSystemObj)))
      (:Is%20Not%20Valid
        _))
    (bind _returnvalue_3 (Niagara|SpawnSystematLocation 0 (Math|Vector|MakeVector _x _y 0.1)))
    (Variables|Default|SetngSystemObj _returnvalue_3)
    (Variables|Default|SetstartMove true)
    (Utilities|FlowControl|Delay 6.0)
    (Variables|Default|SetstartMove false)))

(fn ConstructionScript)