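; Player-controlled Lux character with MOBA-style click-to-move, basic attacks and Q/W/E/R skills.
; Holding right mouse opens a Tick gate that moves to the cursor or attacks clicked pawns in range; range overlaps also trigger attacks.
; Skills share an IsAttacking lock, stop movement, then spawn skill actors with sounds and montages, E at the cursor.
; Wheel zooms the spring arm, and a per-tick camera trace hides blocking actors.
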(event OnComponentBeginOverlap(AttackRange)
  (params (OverlappedComponent :type Primitive%20Component%20Object%20Reference) (OtherActor :type Actor%20Object%20Reference) (OtherComp :type Primitive%20Component%20Object%20Reference) (OtherBodyIndex :type Integer) (bFromSweep :type Boolean) (SweepResult :type Hit%20Result%20Structure%20%28by%20ref%29))
  ;[1 1 1] 우클릭으로 이동 & 평타(사거리 550)
  (Variables|Default|SetEnemy%20In%20Attack%20Range true)
  (CallFunction|Attack))

(event OnComponentEndOverlap(AttackRange)
  (params (OverlappedComponent :type Primitive%20Component%20Object%20Reference) (OtherActor :type Actor%20Object%20Reference) (OtherComp :type Primitive%20Component%20Object%20Reference) (OtherBodyIndex :type Integer))
  ;[1 1 1] 우클릭으로 이동 & 평타(사거리 550)
  (Variables|Default|SetEnemy%20In%20Attack%20Range false))

(event Custom|Damage%20to%20Target
  (bind _state_component_base (Variables|Default|GetState%20Component%20Base))
  (bind _target (Variables|Default|GetTarget))
  (bind _returnvalue (Actor|GetComponentbyClass _target "/Script/InAbyss.StateComponentBase"))
  ;[1 1 1] 우클릭으로 이동 & 평타(사거리 550)
  (Utilities|IsValid _returnvalue
    (:Is%20Valid
      (Class|StateComponentBase|ApplyDamage _returnvalue (Class|StateComponentBase|GetAttackDamage _state_component_base) (Class|StateComponentBase|GetAbilityPower _state_component_base)))))

(event Custom|Attack
  ;[1 1 1] 우클릭으로 이동 & 평타(사거리 550)
  (if (not (Variables|Default|GetIs%20Attacking?))
    (Variables|Default|SetIs%20Attacking? true)
    (Components|Movement|StopMovementImmediately (Variables|Character|GetCharacterMovement))
    (CallFunction|TurnAttackDir)
    (bind _returnvalue (Game|SpawnActorfromClass "/Game/JSH/Blueprints/SKILL/BP_BasicAttack.BP_BasicAttack_C" (Transformation|GetWorldTransform (Variables|Default|GetAttack%20Dir)) "Undefined" "MultiplyWithRoot" 0 0))
    (Variables|/Game/JSH/Blueprints/SKILL/BP_BasicAttack.BP_BasicAttack_C|SetAttackOwner _returnvalue self)
    (Animation|PlayAnimMontage "/Game/JSH/Animations/Montage/lux_attack1_anm_Montage.lux_attack1_anm_Montage" 1.0 "")
    (Utilities|FlowControl|Delay 0.2)
    (Variables|Default|SetIs%20Attacking? false)))

(event EventTick
  (params (DeltaSeconds :type Float%20%28single-precision%29))
  ;[1 1 1] 우클릭으로 이동 & 평타(사거리 550)
  (CallFunction|CameraSystem)
  (Utilities|FlowControl|Gate true
    (:Exit
      (if (not (Variables|Default|GetIs%20Attacking?))
        (CallFunction|TurnAttackDir)
        (bind _clicked_actor (CallFunction|GetClickedActor))
        (Utilities|IsValid _clicked_actor
          (:Is%20Valid
            (Variables|Default|SetTarget _clicked_actor)
            (if (<= (Transformation|GetDistanceTo (Variables|Default|GetTarget)) (Variables|Default|GetAttack%20Distance))
              (CallFunction|Attack)
              (else
                (CallFunction|MovetoActor _clicked_actor))))
          (:Is%20Not%20Valid
            (Variables|Default|SetTarget 0)
            (CallFunction|MovetoClickedPoint)))))))

(event EventBeginPlay
  ;[1 1 1] 마우스 커서 보이기
  (Variables|/Script/Engine.PlayerController|SetbShowMouseCursor (Game|GetPlayerController 0) true))

(event Input|MouseEvents|MouseWheelAxis
  (params (AxisValue :type Float%20%28single-precision%29))
  ;[1 1 1] 마우스 휠로 Zoom in/Out
  (Variables|/Script/Engine.SpringArmComponent|SetTargetArmLength (Variables|Default|GetSpringArm) (Math|Float|Clamp(Float) (+ (* AxisValue -2e+01) (Variables|/Script/Engine.SpringArmComponent|GetTargetArmLength (Variables|Default|GetSpringArm))) 1e+02 1.5e+03)))

(event Input|MouseEvents|RightMouseButton
  (params (Key :type Key%20Structure :default "None"))
  ;[1 1 1] 우클릭으로 이동 & 평타(사거리 550)
  (:Pressed
    (CallFunction|ShowCursorEffect)
    (Utilities|FlowControl|Gate true) ; enters at Open
  )
  (:Released
    (Utilities|FlowControl|Gate true) ; enters at Close
  ))

(event Input|KeyboardEvents|Q
  (params (Key :type Key%20Structure :default "None"))
  ;[1 1 1] 스킬 Q
  (:Pressed
    (if (not (Variables|Default|GetIs%20Attacking?))
      (Variables|Default|SetIs%20Attacking? true)
      (Components|Movement|StopMovementImmediately (Variables|Character|GetCharacterMovement))
      (CallFunction|TurnAttackDir)
      (Utilities|FlowControl|Delay 0.5)
      (Game|SpawnActorfromClass "/Game/JSH/Blueprints/SKILL/BP_QQQ.BP_QQQ_C" (Transformation|GetWorldTransform (Variables|Default|GetAttack%20Dir)) "AlwaysSpawn" "MultiplyWithRoot" 0 0)
      (Collision|SphereOverlapActors "0, 0, 0" 32.0 (Utilities|Array|MakeArray "ObjectTypeQuery3") "/Game/JSH/Blueprints/SKILL/BP_QQQ.BP_QQQ_C")
      (Audio|PlaySound2D "/Game/Resource/LoLResources/Lux/Voice/654029676.654029676" 1.0 1.0 0.0 0 0)
      (bind _returnvalue (Animation|PlayAnimMontage "/Game/JSH/Animations/Montage/lux_spell1_anm_Montage.lux_spell1_anm_Montage" 1.0 "None"))
      (Utilities|FlowControl|Delay _returnvalue)
      (Variables|Default|SetIs%20Attacking? false))))

(event Input|KeyboardEvents|R
  (params (Key :type Key%20Structure :default "None"))
  ;[1 1 1] 스킬 R
  (:Pressed
    (if (not (Variables|Default|GetIs%20Attacking?))
      (Variables|Default|SetIs%20Attacking? true)
      (Components|Movement|StopMovementImmediately (Variables|Character|GetCharacterMovement))
      (CallFunction|TurnAttackDir)
      (Utilities|FlowControl|Delay 0.2)
      (Game|SpawnActorfromClass "/Game/JSH/Blueprints/SKILL/BP_RRR.BP_RRR_C" (Transformation|GetWorldTransform (Variables|Default|GetAttack%20Dir)) "AlwaysSpawn" "MultiplyWithRoot" 0 0)
      (Audio|PlaySound2D "/Game/Resource/LoLResources/Lux/Voice/620310710.620310710" 1.0 1.0 0.0 0 0)
      (bind _returnvalue (Animation|PlayAnimMontage "/Game/JSH/Animations/Montage/lux_spell4_anm_Montage.lux_spell4_anm_Montage" 1.0 "None"))
      (Utilities|FlowControl|Delay _returnvalue)
      (Variables|Default|SetIs%20Attacking? false))))

(event Input|KeyboardEvents|W
  (params (Key :type Key%20Structure :default "None"))
  ;[1 1 1] 스킬 W
  (:Pressed
    (if (not (Variables|Default|GetIs%20Attacking?))
      (Variables|Default|SetIs%20Attacking? true)
      (Components|Movement|StopMovementImmediately (Variables|Character|GetCharacterMovement))
      (CallFunction|TurnAttackDir)
      (Utilities|FlowControl|Delay 0.2)
      (bind _returnvalue (Game|SpawnActorfromClass "/Game/JSH/Blueprints/SKILL/BP_Barrier.BP_Barrier_C" (Math|Transform|MakeTransform (Transformation|GetActorLocation) "0, 0, 0" "1.000000,1.000000,1.000000") "AlwaysSpawn" "MultiplyWithRoot" 0 0))
      (Transformation|AttachActorToActor _returnvalue self "None" "SnapToTarget" "SnapToTarget" "KeepWorld" true)
      (bind _returnvalue_2 (Game|SpawnActorfromClass "/Game/JSH/Blueprints/SKILL/BP_WWW.BP_WWW_C" (Transformation|GetWorldTransform (Variables|Default|GetAttack%20Dir)) "AlwaysSpawn" "MultiplyWithRoot" 0 0))
      (Variables|/Game/JSH/Blueprints/SKILL/BP_WWW.BP_WWW_C|SetOwningPlayer _returnvalue_2 self)
      (Audio|PlaySound2D "/Game/Resource/LoLResources/Lux/Voice/1742609802.1742609802" 1.0 1.0 0.0 0 0)
      (bind _returnvalue_3 (Animation|PlayAnimMontage "/Game/JSH/Animations/Montage/lux_spell2_anm_Montage.lux_spell2_anm_Montage" 1.0 "None"))
      (Utilities|FlowControl|Delay _returnvalue_3)
      (Variables|Default|SetIs%20Attacking? false))))

(event Input|KeyboardEvents|E
  (params (Key :type Key%20Structure :default "None"))
  ;[1 1 1] 스킬 E
  (:Pressed
    (if (not (Variables|Default|GetIs%20Attacking?))
      (Variables|Default|SetIs%20Attacking? true)
      (Components|Movement|StopMovementImmediately (Variables|Character|GetCharacterMovement))
      (CallFunction|TurnAttackDir)
      (Utilities|FlowControl|Delay 0.2)
      (Game|SpawnActorfromClass "/Game/JSH/Blueprints/SKILL/BP_E.BP_E_C" (Math|Transform|MakeTransform (.Location (Collision|BreakHitResult (.HitResult (Game|Player|GetHitResultUnderCursorbyChannel (Game|GetPlayerController 0) "TraceTypeQuery1" true))))) "AlwaysSpawn" "MultiplyWithRoot" 0 0)
      (Collision|SphereOverlapActors "0, 0, 0" 32.0 (Utilities|Array|MakeArray "ObjectTypeQuery3") "/Game/JSH/Blueprints/SKILL/BP_QQQ.BP_QQQ_C")
      (Audio|PlaySound2D "/Game/Resource/LoLResources/Lux/Voice/1399447772.1399447772" 1.0 1.0 0.0 0 0)
      (bind _returnvalue (Animation|PlayAnimMontage "/Game/JSH/Animations/Montage/lux_spell3_anm_Montage.lux_spell3_anm_Montage" 1.0 "None"))
      (Utilities|FlowControl|Delay _returnvalue)
      (Variables|Default|SetIs%20Attacking? false))))

(fn ConstructionScript)

(fn GetClickedActor
  (bind _returnvalue (Game|GetPlayerController 0))
  (bind _array (Utilities|Array|MakeArray "ObjectTypeQuery3"))
  (bind _hitresult (Class|PlayerController|GetHitResultUnderCursorforObjects _returnvalue _array true))
  (if (== (.hitactor _hitresult) self)
    (return 0)
    (else
      (return (.hitactor _hitresult)))))

(fn MovetoActor
  (params (Move%20to%20Actor :type Actor%20Object%20Reference))
  (AI|Navigation|SimpleMovetoActor (Game|GetPlayerController 0) Move%20to%20Actor))

(fn GetDestinationtoMove
  (return (.location (.HitResult (Game|Player|GetHitResultUnderCursorbyChannel (Game|GetPlayerController 0) "TraceTypeQuery1" true)))))

(fn MovetoClickedPoint
  (bind _charactermovement (Variables|Character|GetCharacterMovement))
  (bind _destination (CallFunction|GetDestinationtoMove))
  (Variables|Default|SetMove%20Destination _destination)
  (if (> (Math|Vector|VectorLength (- (Variables|Default|GetMove%20Destination) (Transformation|GetActorLocation))) 1.5e+02)
    (Variables|/Script/Engine.CharacterMovementComponent|SetMaxWalkSpeed _charactermovement 6e+02)
    (else
      (Variables|/Script/Engine.CharacterMovementComponent|SetMaxWalkSpeed _charactermovement 3e+02)))
  (AI|Navigation|SimpleMovetoLocation (Game|GetPlayerController 0) (Variables|Default|GetMove%20Destination)))

(fn TurnAttackDir
  (bind _returnvalue (Game|GetPlayerController 0))
  (bind (_worldlocation _worlddirection) (Game|Player|ConvertMouseLocationToWorldSpace _returnvalue))
  (bind (_outhit _returnvalue_2) (Collision|LineTraceByChannel _worldlocation (+ _worldlocation (* _worlddirection 3e+04)) "TraceTypeQuery1" false 0 "None"))
  (if _returnvalue_2
    (bind _output_get (Variables|Default|SetDirection (- (.Location (Collision|BreakHitResult _outhit)) (Transformation|GetActorLocation))))
    (AI|Navigation|SimpleMovetoLocation (Pawn|GetController) (Transformation|GetActorLocation))))

(fn CameraSystem
  (bind (_outhit _returnvalue) (Collision|LineTraceByChannel (Transformation|GetWorldLocation (Variables|Default|GetCamera)) (+ (Transformation|GetWorldLocation (Variables|Character|GetMesh)) "0.000000,0.000000,200.000000") "TraceTypeQuery2" false (Utilities|Array|MakeArray 0) "None"))
  (if _returnvalue
    (bind _cameraobstacle (Variables|Default|GetCameraObstacle)
      (:then
        (if (not (== _cameraobstacle (.HitActor (Collision|BreakHitResult _outhit))))
          (Rendering|SetActorHiddenInGame _cameraobstacle false)
          (bind _output_get (Variables|Default|SetCameraObstacle (.HitActor (Collision|BreakHitResult _outhit)) :!label _label))
          (Rendering|SetActorHiddenInGame _output_get true)))
      (:else
        (goto _label)))
    (else
      (bind _cameraobstacle_2 (Variables|Default|GetCameraObstacle)
        (:then
          (Rendering|SetActorHiddenInGame _cameraobstacle_2 false))
        (:else)))))

(fn ShowCursorEffect
  (bind _clicked_actor (CallFunction|GetClickedActor))
  (Utilities|IsValid _clicked_actor
    (:Is%20Not%20Valid
      (Niagara|SpawnSystematLocation (Variables|Default|GetFX_MouseCursor) (.location (.HitResult (Game|Player|GetHitResultUnderCursorbyChannel (Game|GetPlayerController 0) "TraceTypeQuery1" true)))))))

(fn RotatetoTargetRotation
  (params (DeltaTime :type Float%20%28double-precision%29))
  (bind _returnvalue (Transformation|GetActorRotation))
  (if (not (Utilities|Operators|EqualEqual _returnvalue (Variables|Default|GetTargetRotation) 0.1))
    (Transformation|SetActorRotation (Math|Rotator|Lerp(Rotator) _returnvalue (Variables|Default|GetTargetRotation) (* DeltaTime (Variables|Default|GetRotateSpeed)) true))))