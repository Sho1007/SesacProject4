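; Playable Lux character with MOBA-style controls: visible cursor, right-click move and attack, and wheel-driven camera zoom.
; Right-click traces under the cursor and issues AIMoveTo, then attacks or approaches any clicked pawn depending on the AttackRange overlap flag.
; A Character entering AttackRange also triggers Attack, which halts movement and plays a montage behind an IsAttacking guard.
; QWER only play spell montages; no damage is applied.
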(event OnComponentBeginOverlap(AttackRange)
  (params (OverlappedComponent :type Primitive%20Component%20Object%20Reference) (OtherActor :type Actor%20Object%20Reference) (OtherComp :type Primitive%20Component%20Object%20Reference) (OtherBodyIndex :type Integer) (bFromSweep :type Boolean) (SweepResult :type Hit%20Result%20Structure%20%28by%20ref%29))
  (Utilities|Casting|CastToCharacter OtherActor)
  (Variables|Default|SetEnemy%20In%20Attack%20Range true)
  (CallFunction|Attack))

(event OnComponentEndOverlap(AttackRange)
  (params (OverlappedComponent :type Primitive%20Component%20Object%20Reference) (OtherActor :type Actor%20Object%20Reference) (OtherComp :type Primitive%20Component%20Object%20Reference) (OtherBodyIndex :type Integer))
  (Utilities|Casting|CastToCharacter OtherActor)
  (Variables|Default|SetEnemy%20In%20Attack%20Range false))

(event Custom|Attack
  (if (not (Variables|Default|GetIs%20Attacking?))
    (Variables|Default|SetIs%20Attacking? true)
    (Components|Movement|StopMovementImmediately (Variables|Character|GetCharacterMovement))
    (bind _returnvalue (Animation|PlayAnimMontage "/Game/Resource/LoLResources/Lux/Animations/lux_attack1_anm_Montage.lux_attack1_anm_Montage" 1.0 "None"))
    (Utilities|FlowControl|Delay _returnvalue)
    (Variables|Default|SetIs%20Attacking? false)))

(event EventBeginPlay
  ;[1 1 1] 마우스 커서 보이기
  (Variables|/Script/Engine.PlayerController|SetbShowMouseCursor (Game|GetPlayerController 0) true))

(event Input|MouseEvents|MouseWheelAxis
  (params (AxisValue :type Float%20%28single-precision%29))
  ;[1 1 1] 마우스 휠로 Zoom in/Out
  (Variables|/Script/Engine.SpringArmComponent|SetTargetArmLength (Variables|Default|GetSpringArm) (Math|Float|Clamp(Float) (+ (* AxisValue -2e+01) (Variables|/Script/Engine.SpringArmComponent|GetTargetArmLength (Variables|Default|GetSpringArm))) 5e+01 1e+03)))

(event Input|KeyboardEvents|Q
  (params (Key :type Key%20Structure :default "None"))
  ;[1 1 1] QWER 스킬 애니메이션
  (:Pressed
    (Animation|Montage|PlayMontage (Variables|Character|GetMesh) "/Game/Resource/LoLResources/Lux/Animations/lux_spell1_anm_Montage.lux_spell1_anm_Montage")))

(event Input|MouseEvents|RightMouseButton
  (params (Key :type Key%20Structure :default "None"))
  (bind _returnvalue (Game|GetPlayerController 0))
  (bind (_worldlocation _worlddirection) (Game|Player|ConvertMouseLocationToWorldSpace _returnvalue))
  ;[1 1 1] 우클릭으로 이동 & Attack
  (:Pressed
    (bind (_outhit _returnvalue_2) (Collision|LineTraceByChannel _worldlocation (+ _worldlocation (* _worlddirection 1e+03)) "TraceTypeQuery1" false 0 "None"))
    (if _returnvalue_2
      (AI|AIMoveTo (Pawn|GetController) self (.Location (Collision|BreakHitResult _outhit)) 0 5.0 false
        (:then
          (bind _clicked_actor (CallFunction|GetClickedActor))
          (Utilities|IsValid _clicked_actor
            (:Is%20Valid
              (if (Variables|Default|GetEnemy%20In%20Attack%20Range)
                (CallFunction|Attack)
                (else
                  (CallFunction|MovetoActor _clicked_actor))))))))))

(event Input|KeyboardEvents|W
  (params (Key :type Key%20Structure :default "None"))
  ;[1 1 1] QWER 스킬 애니메이션
  (:Pressed
    (Animation|Montage|PlayMontage (Variables|Character|GetMesh) "/Game/Resource/LoLResources/Lux/Animations/lux_spell2_anm_Montage.lux_spell2_anm_Montage")))

(event Input|KeyboardEvents|E
  (params (Key :type Key%20Structure :default "None"))
  ;[1 1 1] QWER 스킬 애니메이션
  (:Pressed
    (Animation|Montage|PlayMontage (Variables|Character|GetMesh) "/Game/Resource/LoLResources/Lux/Animations/lux_spell3_anm_Montage.lux_spell3_anm_Montage")))

(event Input|KeyboardEvents|R
  (params (Key :type Key%20Structure :default "None"))
  ;[1 1 1] QWER 스킬 애니메이션
  (:Pressed
    (Animation|Montage|PlayMontage (Variables|Character|GetMesh) "/Game/Resource/LoLResources/Lux/Animations/lux_spell4_anm_Montage.lux_spell4_anm_Montage")))

(fn ConstructionScript)

(fn GetClickedActor
  (return (.hitactor (.HitResult (Class|PlayerController|GetHitResultUnderCursorforObjects (Game|GetPlayerController 0) (Utilities|Array|MakeArray "ObjectTypeQuery3") true)))))

(fn MovetoActor
  (params (Move%20to%20Actor :type Actor%20Object%20Reference))
  (AI|Navigation|SimpleMovetoActor (Game|GetPlayerController 0) Move%20to%20Actor))